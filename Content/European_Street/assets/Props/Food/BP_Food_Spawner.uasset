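; Food spawner prop Blueprint that shows a random food mesh: donut, cake or croissant, according to its TypeOfFood setting.
; The construction script selects the matching collection from Food, converts it to an array and assigns a random entry to the Sphere mesh component.
; The random index is bounded by length minus one, so the last entry is never picked when a collection holds several meshes.
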(fn ConstructionScript
  (bind _food (Variables|Default|GetFood))
  (bind _type_of_food (Variables|Default|GetType%20of%20Food))
  (bind (_donats _cakes _croissant) (Utilities|Struct|BreakBS_Food _food))
  (bind _returnvalue (Utilities|Select :Index _type_of_food :NewEnumerator0 _donats :NewEnumerator1 _cakes :NewEnumerator2 _croissant))
  (bind _result (Utilities|Set|ToArray _returnvalue))
  (Components|StaticMesh|SetStaticMesh (Variables|Default|GetSphere) (Utilities|Array|Get(acopy) _result (Math|Random|RandomInteger (- (Utilities|Set|Length _returnvalue) 1)))))